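; Clickable cube actor with a widget component, apparently an in-world entry point for a room inventory UI.
; Clicking the cube creates a WBP_RoomInv widget without adding it to the viewport and prints a debug "Hello".
; Cursor hover sets Isactive false before branching on it, so it always deactivates the widget component.
; The branch that would activate the hovered component and turn the widget toward the camera never runs.
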(event OnClicked(Cube)
  (params (TouchedComponent :type Primitive%20Component%20Object%20Reference) (ButtonPressed :type Key%20Structure :default "None"))
  (UserInterface|CreateWidget "/Game/Loic/WBP_RoomInv.WBP_RoomInv_C")
  (Development|PrintString "Hello"))

(event OnBeginCursorOver(Cube)
  (params (TouchedComponent :type Primitive%20Component%20Object%20Reference))
  (Variables|Default|SetIsactive false)
  (if (Variables|Default|GetIsactive)
    (Components|Activation|Activate TouchedComponent false)
    (Transformation|SetWorldTransform (Variables|Default|GetWidget) (Math|Transform|MakeTransform "0, 0, 0" (Math|Rotator|FindLookatRotation (Transformation|GetWorldLocation (Variables|Default|GetScene)) (Camera|GetCameraLocation (Game|GetPlayerCameraManager 0))) "1.000000,1.000000,1.000000") false false)
    (else
      (Components|Activation|Deactivate (Variables|Default|GetWidget)))))

(event EventBeginPlay)

(event Collision|EventActorBeginOverlap
  (params (OtherActor :type Actor%20Object%20Reference)))

(event EventTick
  (params (DeltaSeconds :type Float%20%28single-precision%29)))

(fn ConstructionScript)